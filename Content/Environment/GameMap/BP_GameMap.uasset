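; Procedural game map actor that builds, on the authority, a seeded grid of BP_MapTile child actors with varying height and void tiles.
; CreateGridArray picks each height within a slope limit of neighbouring tiles, advancing a working seed per tile for BuildMapGrid to spawn.
; A weighted seeded pass then places TreeStump blockages on non-void tiles.
; RegenerateMap rebuilds everything from new parameters, and SetAtmosphere pushes the environment type to all tiles.
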(event `PlaceBlockageOnTile`
  (params (Tile :type "/Game/Environment/GameMap/BP_MapTile Object Reference") (BlockageClass :type "/Game/Environment/TilePlacement/Blockage Class Reference"))
  (bind _returnvalue (`|SpawnActorFromClass` BlockageClass (`self.GetTransform` Tile) "AlwaysSpawn" "OverrideRootScale" null null))
  (set `/Game/Environment/GameMap/BP_MapTile.Blockage` _returnvalue Tile))

(event `self.ReceiveBeginPlay`
  (set `self.WorkingSeed` (`self.InitialSeed`))
  (`/Engine/EditorBlueprintResources/ActorMacros.Switch Has Authority` :!label _label
    (:`Authority`
      (`self.BuildMapGrid`)
      (`self.PlaceMidpoint`)
      (bind _outactors (`GameplayStatics.GetAllActorsOfClass` "/Game/Environment/GameMap/BP_MapTile.BP_MapTile_C"))
      (for _array_element _outactors
        (if (and (`KismetMathLibrary.RandomBoolWithWeightFromStream` (`self.BlockageWeight`) (`KismetMathLibrary.MakeRandomStream` (`self.WorkingSeed`))) (not (`/Game/Environment/GameMap/BP_MapTile.Void` _array_element)))
          (`self.PlaceBlockageOnTile` _array_element "/Game/Environment/TilePlacement/Blockages/TreeStump.TreeStump_C"))
        (set `self.WorkingSeed` (`KismetMathLibrary.RandomIntegerInRangeFromStream` 0 999999 (`KismetMathLibrary.MakeRandomStream` (`self.WorkingSeed`))))))))

(event `RegenerateMap`
  (params (NewSeed :type Integer) (MaxTileHeight :type "Float (double-precision)") (MaxSlopeHeight :type "Float (double-precision)") (VoidWeight :type "Float (double-precision)") (BlockageWeight :type "Float (double-precision)"))
  (`self.DestroyMap`)
  (set `self.WorkingSeed` (`KismetMathLibrary.Clamp` NewSeed 0 999999))
  (set `self.MaxTileHeight` MaxTileHeight)
  (set `self.MaxSlopeHeight` MaxSlopeHeight)
  (set `self.VoidWeight` VoidWeight)
  (set `self.BlockageWeight` BlockageWeight)
  (goto _label))

(fn `BuildMapGrid`
  (`self.CreateGridArray`)
  (for (_array_element _array_index) (`self.TileGrid`)
    (bind _tilearray (break `/Game/Environment/GameMap/TileRow` _array_element))
    (for (_array_element_2 _array_index_2) _tilearray
      (bind (_tilereference _height _void) (break `/Game/Environment/GameMap/TileData` _array_element_2))
      (bind _returnvalue (`AddComponent|NODE_AddChildActorComponent-0` :`RelativeTransform` (`KismetMathLibrary.MakeTransform` (* (`KismetMathLibrary.MakeVector` (`KismetMathLibrary.Conv_IntToDouble` _array_index) (`KismetMathLibrary.Conv_IntToDouble` _array_index_2) _height) 100.0))))
      (`ChildActorComponent.SetChildActorClass` _returnvalue "/Game/Environment/GameMap/BP_MapTile.BP_MapTile_C")
      (bind _asbp_map_tile (cast `/Game/Environment/GameMap/BP_MapTile` (`ChildActorComponent.ChildActor` _returnvalue)))
      (`/Game/Environment/GameMap/BP_MapTile.SetCoordinates` _asbp_map_tile self _array_index _array_index_2)
      (`/Game/Environment/GameMap/BP_MapTile.SetAtmosphere` _asbp_map_tile (`self.EnvironmentType`))
      (`/Game/Environment/GameMap/BP_MapTile.SetVoid` _asbp_map_tile _void)
      (`KismetArrayLibrary.Array_Set` _tilearray _array_index_2 (make `/Game/Environment/GameMap/TileData` _asbp_map_tile _height _void)))))

(fn `CreateGridArray`
  (bind _maxslopeheight (`self.MaxSlopeHeight`))
  (bind _returnvalue (`KismetMathLibrary.MakeRandomStream` (`self.WorkingSeed`)))
  (set `self.SetUpInProgress` true)
  (for _index (range (`self.Rows`))
    (`KismetArrayLibrary.Array_Clear` (`self.ColumnSetupArray`))
    (set `self.RowBeingSetUp` _index)
    (for _index_2 (range (`self.Columns`))
      (bind (_averageheight _tallest _shortest) (`self.GetNeighbouringTileAverageHeight` _index _index_2))
      (`KismetArrayLibrary.Array_Add` (`self.ColumnSetupArray`) (make `/Game/Environment/GameMap/TileData` null (`KismetMathLibrary.RandomFloatInRangeFromStream` (`KismetMathLibrary.FClamp` (- _shortest _maxslopeheight) 0.0 (`self.MaxTileHeight`)) (`KismetMathLibrary.FClamp` (+ _maxslopeheight _tallest) 0.0 (`self.MaxTileHeight`)) _returnvalue) (`KismetMathLibrary.RandomBoolWithWeightFromStream` (`self.VoidWeight`) _returnvalue)))
      (set `self.WorkingSeed` (`KismetMathLibrary.RandomIntegerInRangeFromStream` 0 999999 (`KismetMathLibrary.MakeRandomStream` (`self.WorkingSeed`)))))
    (`KismetArrayLibrary.Array_Add` (`self.TileGrid`) (make `/Game/Environment/GameMap/TileRow` (`self.ColumnSetupArray`))))
  (set `self.SetUpInProgress` false))

(fn `DestroyMap`
  (bind _outactors (`GameplayStatics.GetAllActorsOfClass` "/Game/Environment/GameMap/BP_MapTile.BP_MapTile_C"))
  (for _array_element _outactors
    (`self.K2_DestroyActor` _array_element))
  (bind _outactors_2 (`GameplayStatics.GetAllActorsOfClass` "/Game/Environment/TilePlacement/Blockage.Blockage_C"))
  (for _array_element_2 _outactors_2
    (`self.K2_DestroyActor` _array_element_2))
  (`KismetArrayLibrary.Array_Clear` (`self.TileGrid`)))

(fn `DoesTileExist`
  (params (TileX :type Integer) (TileY :type Integer))
  (returns (TileData :type Boolean))
  (bind _tilegrid (`self.TileGrid`))
  (bind _returnvalue (`KismetArrayLibrary.Array_Length` (`self.ColumnSetupArray`)))
  (bind _returnvalue_2 (- (`KismetArrayLibrary.Array_Length` _tilegrid) 1))
  (bind _returnvalue_3 (`KismetArrayLibrary.Array_Length` (`.TileArray_3_8686633D4C350C3FF21D7096EBAAFD56` (break `/Game/Environment/GameMap/TileRow` (`|GetArrayItem` _tilegrid TileX)))))
  (if (and (`self.SetUpInProgress`) (== TileX (`self.RowBeingSetUp`)))
    (if (and (>= TileY 0) (<= TileY (- _returnvalue 1)) (> _returnvalue 0))
      (return true)
      (else
        (return false)))
    (else
      (if (and (>= TileX 0) (<= TileX _returnvalue_2) (> _returnvalue_2 0))
        (if (and (>= TileY 0) (<= TileY (- _returnvalue_3 1)) (> _returnvalue_3 0))
          (return true)
          (else
            _)))
      (return false))))

(fn `GetNeighbouringTileAverageHeight`
  (params (TileX :type Integer) (TileY :type Integer))
  (returns (AverageHeight :type "Float (double-precision)") (Tallest :type "Float (double-precision)") (Shortest :type "Float (double-precision)"))
  (locals (RefX :type Integer) (RefY :type Integer) (TilesChecked :type Integer) (TotalHeight :type "Float (double-precision)") (TallestTile :type "Float (double-precision)") (ShortestTile :type "Float (double-precision)") (CurrentTileHeight :type "Float (double-precision)"))
  (bind _currenttileheight (`local.CurrentTileHeight`))
  (bind _currenttileheight_2 (`local.CurrentTileHeight`))
  (set `local.RefX` TileX)
  (set `local.RefY` TileY)
  (`|ExecutionSequence`
    (:`then_0`
      (bind _tiledata (`self.GetTileDataAtCoordinates` (- (`local.RefX`) 1) (`local.RefY`)))
      (bind (_tilereference _height) (break `/Game/Environment/GameMap/TileData` _tiledata))
      (set `local.CurrentTileHeight` _height)
      (set `local.TotalHeight` (+ _height (`local.TotalHeight`)))
      (`/Engine/EditorBlueprintResources/StandardMacros.IncrementInt` (`local.TilesChecked`)
        (:`  `
          (if (or (< (`local.TallestTile`) 0.0) (< (`local.ShortestTile`) 0.0)) :!label _label
            (set `local.TallestTile` _currenttileheight_2)
            (set `local.ShortestTile` _currenttileheight_2)
            (elif (> _currenttileheight (`local.TallestTile`))
              (set `local.TallestTile` _currenttileheight)
              (elif (< _currenttileheight (`local.ShortestTile`))
                (set `local.ShortestTile` _currenttileheight)))))))
    (:`then_1`
      (bind _tiledata_2 (`self.GetTileDataAtCoordinates` (`local.RefX`) (- (`local.RefY`) 1)))
      (bind (_tilereference_2 _height_2) (break `/Game/Environment/GameMap/TileData` _tiledata_2))
      (set `local.CurrentTileHeight` _height_2)
      (set `local.TotalHeight` (+ _height_2 (`local.TotalHeight`)))
      (`/Engine/EditorBlueprintResources/StandardMacros.IncrementInt` (`local.TilesChecked`)
        (:`  `
          (goto _label))))
    (:`then_2`
      (bind _tiledata_3 (`self.GetTileDataAtCoordinates` (+ (`local.RefX`) 1) (`local.RefY`)))
      (bind (_tilereference_3 _height_3) (break `/Game/Environment/GameMap/TileData` _tiledata_3))
      (set `local.CurrentTileHeight` _height_3)
      (set `local.TotalHeight` (+ _height_3 (`local.TotalHeight`)))
      (`/Engine/EditorBlueprintResources/StandardMacros.IncrementInt` (`local.TilesChecked`)
        (:`  `
          (if (> _height_3 (`local.TallestTile`))
            (set `local.TallestTile` _height_3)
            (elif (< _height_3 (`local.ShortestTile`))
              (set `local.ShortestTile` _height_3)
              (goto _label))))))
    (:`then_3`
      (bind _tiledata_4 (`self.GetTileDataAtCoordinates` (`local.RefX`) (+ (`local.RefY`) 1)))
      (bind (_tilereference_4 _height_4) (break `/Game/Environment/GameMap/TileData` _tiledata_4))
      (set `local.CurrentTileHeight` _height_4)
      (set `local.TotalHeight` (+ _height_4 (`local.TotalHeight`)))
      (`/Engine/EditorBlueprintResources/StandardMacros.IncrementInt` (`local.TilesChecked`)
        (:`  `
          (if (> _height_4 (`local.TallestTile`))
            (set `local.TallestTile` _height_4)
            (elif (< _height_4 (`local.ShortestTile`))
              (set `local.ShortestTile` _height_4)
              (goto _label))))))
    (:`then_4`
      (if (> (`local.TilesChecked`) 0)
        (return (/ (`local.TotalHeight`) (`KismetMathLibrary.Conv_IntToDouble` (`local.TilesChecked`))) (`local.TallestTile`) (`local.ShortestTile`))
        (else
          (`KismetSystemLibrary.PrintText` (`|FormatText` "{x} {y}" (`local.RefX`) (`local.RefY`)))
          (return (`KismetMathLibrary.RandomFloatInRange` 0.0 (`self.MaxTileHeight`)) (`self.MaxTileHeight`) 0.0))))))

(fn `GetTileDataAtCoordinates`
  (params (TileX :type Integer) (TileY :type Integer))
  (returns (TileData :type "/Game/Environment/GameMap/TileData Structure"))
  (if (and (`self.SetUpInProgress`) (== TileX (`self.RowBeingSetUp`)))
    (return (`|GetArrayItem` (`self.ColumnSetupArray`) TileY))
    (else
      (return (`|GetArrayItem` (`.TileArray_3_8686633D4C350C3FF21D7096EBAAFD56` (break `/Game/Environment/GameMap/TileRow` (`|GetArrayItem` (`self.TileGrid`) TileX))) TileY)))))

(fn `PlaceMidpoint`
  (`SceneComponent.K2_SetRelativeLocation` (`self.Midpoint`) (`KismetMathLibrary.MakeVector` (`KismetMathLibrary.Conv_IntToDouble` (- (* (`self.Rows`) 50) 50)) (`KismetMathLibrary.Conv_IntToDouble` (- (* (`self.Columns`) 50) 50))) false false))

(fn `SetAtmosphere`
  (params (EnvironmentType :type "EEnvironmentEnum Enum" :default "Env_Woodlands"))
  (set `self.EnvironmentType` EnvironmentType)
  (bind _outactors (`GameplayStatics.GetAllActorsOfClass` "/Game/Environment/GameMap/BP_MapTile.BP_MapTile_C"))
  (for _array_element _outactors
    (`/Game/Environment/GameMap/BP_MapTile.SetAtmosphere` _array_element EnvironmentType)))

(fn `UserConstructionScript`)