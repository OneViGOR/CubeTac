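; Grid tile for the tactical game map, holding coordinates, occupant and movement cost including any blockage.
; Clicks route by game phase to portal placement, or to moving, ability use, portal spawning and character selection through the player's controller and pawn.
; Hover refreshes a child Marker actor, a data table sets environment materials, and Void tiles are hidden and ignore Visibility traces.
; Downward line traces at fixed offsets find the four neighbouring tiles.
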(event `self.ReceiveBeginPlay`
  (`self.SetVoid` (`self.Void`)))

(event `SetOccupyingCharacter`
  (params (OccupyingCharacter :type "/Game/CharacterData/GridCharacter Object Reference"))
  (set `self.OccupyingCharacter` OccupyingCharacter))

(event `self.ReceiveActorBeginCursorOver`
  (if (`|EnumInequality` (`/Game/GameData/TacticalGameState_Old.GamePhase` (cast `/Game/GameData/TacticalGameState_Old` (`GameplayStatics.GetGameState`) :!pure true)) "NewEnumerator2")
    (set `self.MouseOver` true)
    (`self.SetHighlightMaterial`)))

(event `SetAtmosphere`
  (params (Environment :type "EEnvironmentEnum Enum" :default "Env_Woodlands"))
  (bind _returnvalue (`|GetDataTableRow` "/Game/Environment/Environment/EnvironmentColours.EnvironmentColours" (`KismetStringLibrary.Conv_StringToName` (`|GetEnumeratorNameAsString` Environment)))
    (:`then`
      (bind (_skymaterial _fogcolour _tilecapmaterial _tileshaftmaterial) (break `Environment` _returnvalue))
      (`PrimitiveComponent.SetMaterial` (`self.Cap`) 0 _tilecapmaterial)
      (`PrimitiveComponent.SetMaterial` (`self.Shaft`) 0 _tileshaftmaterial))))

(event `self.ReceiveActorEndCursorOver`
  (if (`|EnumInequality` (`/Game/GameData/TacticalGameState_Old.GamePhase` (cast `/Game/GameData/TacticalGameState_Old` (`GameplayStatics.GetGameState`) :!pure true)) "NewEnumerator2")
    (set `self.MouseOver` false)
    (`self.SetHighlightMaterial`)))

(event `self.ReceiveActorOnClicked`
  (params (ButtonPressed :type "Key Structure"))
  (if (not (`self.Void`))
    (switch `/Game/GameData/GamePhase` (`/Game/GameData/TacticalGameState_Old.GamePhase` (cast `/Game/GameData/TacticalGameState_Old` (`GameplayStatics.GetGameState`) :!pure true))
      (:`NewEnumerator0`
        (`self.ClickedInPortalPlacementPhase`))
      (:`NewEnumerator1`
        (`self.ClickedInGamePhase`)))))

(event `SetVoid`
  (params (Void :type Boolean))
  (bind _cap (`self.Cap`))
  (bind _cap_2 (`self.Cap`))
  (bind _output_get (set `self.Void` Void))
  (if _output_get
    (`SceneComponent.SetVisibility` _cap_2 false false)
    (`SceneComponent.SetVisibility` (`self.Shaft`) false false)
    (`SceneComponent.SetVisibility` (`self.Marker`) false false)
    (`SceneComponent.SetVisibility` (`self.CoordinateText`) false false)
    (`PrimitiveComponent.SetCollisionResponseToChannel` _cap_2 "ECC_Visibility" "ECR_Ignore")
    (`PrimitiveComponent.SetCollisionResponseToChannel` (`self.Shaft`) "ECC_Visibility" "ECR_Ignore")
    (else
      (`SceneComponent.SetVisibility` _cap true false)
      (`SceneComponent.SetVisibility` (`self.Shaft`) true false)
      (`SceneComponent.SetVisibility` (`self.CoordinateText`) true false)
      (`SceneComponent.SetVisibility` (`self.Marker`) true false)
      (`PrimitiveComponent.SetCollisionResponseToChannel` _cap "ECC_Visibility" "ECR_Block")
      (`PrimitiveComponent.SetCollisionResponseToChannel` (`self.Shaft`) "ECC_Visibility" "ECR_Block"))))

(fn `ClickedInGamePhase`
  (bind _occupyingcharacter (`self.OccupyingCharacter`))
  (bind _astactical_controller_old (cast `/Game/Player/TacticalController_Old` (`GameplayStatics.GetPlayerController` 0) :!pure true))
  (if (`|EnumInequality` (`self.CurrentlyNavigable`) "NewEnumerator2")
    (`/Game/Player/PlayerPawn_Old.MoveCharacter` (cast `/Game/Player/PlayerPawn_Old` (`Controller.K2_GetPawn` _astactical_controller_old) :!pure true) self _astactical_controller_old)
    (else
      (bind _astactical_controller_old_2 (cast `/Game/Player/TacticalController_Old` (`GameplayStatics.GetPlayerController` 0)))
      (bind _selectedcharacter (`/Game/Player/TacticalController_Old.SelectedCharacter` _astactical_controller_old_2))
      (`/Engine/EditorBlueprintResources/StandardMacros.IsValid` _selectedcharacter
        (:`Is Valid`
          (if (`self.Targetable`)
            (bind (_asportal _bsuccess) (cast `/Game/Environment/TilePlacement/Portal` _selectedcharacter :!pure true))
            (if _bsuccess
              (`/Game/Environment/TilePlacement/Portal.SpawnCharacter` _asportal self)
              (else
                (`/Game/CharacterData/GridCharacter.UseSelectedAbility` _selectedcharacter self)))
            (else
              (`/Game/CharacterData/GridCharacter.DeselectCharacter` _selectedcharacter)
              (`/Engine/EditorBlueprintResources/StandardMacros.IsValid` _occupyingcharacter :!label _label
                (:`Is Valid`
                  (if (== (`/Game/CharacterData/GridCharacter.Team` _occupyingcharacter) (`/Game/Player/TacticalController_Old.Team` _astactical_controller_old_2))
                    (`/Game/CharacterData/GridCharacter.SelectCharacter` _occupyingcharacter)))))))
        (:`Is Not Valid`
          (goto _label))))))

(fn `ClickedInPortalPlacementPhase`
  (bind _astactical_controller_old (cast `/Game/Player/TacticalController_Old` (`GameplayStatics.GetPlayerController` 0)))
  (if (and (`/Game/Player/TacticalController_Old.Turn` _astactical_controller_old) (not (`KismetSystemLibrary.IsValid` (`self.Blockage`))))
    (bind _ownedportal (`/Game/Player/TacticalController_Old.OwnedPortal` _astactical_controller_old))
    (`/Engine/EditorBlueprintResources/StandardMacros.IsValid` _ownedportal
      (:`Is Valid`
        (bind _asplayer_pawn_old (cast `/Game/Player/PlayerPawn_Old` (`Controller.K2_GetPawn` _astactical_controller_old) :!pure true))
        (`/Game/Player/PlayerPawn_Old.DestroyActor` _asplayer_pawn_old _ownedportal))
      (:`Is Not Valid`
        _))
    (`/Game/Player/PlayerPawn_Old.SpawnPortal` _asplayer_pawn_old self (`/Game/Player/TacticalController_Old.Team` _astactical_controller_old))))

(fn `GetFourNeighbouringTiles`
  (returns (Tiles :type "Array of /Game/Environment/GameMap/BP_MapTile Object Reference"))
  (locals (TilesFound :type "Array of /Game/Environment/GameMap/BP_MapTile Object Reference"))
  (`|ExecutionSequence`
    (:`then_0`
      (bind (_success _tile) (`self.LineTraceForTile` (+ (`self.K2_GetActorLocation`) (100.0 0.0 0.0))))
      (if _success
        (`KismetArrayLibrary.Array_Add` (`local.TilesFound`) _tile)))
    (:`then_1`
      (bind (_success_2 _tile_2) (`self.LineTraceForTile` (+ (`self.K2_GetActorLocation`) (-100.0 0.0 0.0))))
      (if _success_2
        (`KismetArrayLibrary.Array_Add` (`local.TilesFound`) _tile_2)))
    (:`then_2`
      (bind (_success_3 _tile_3) (`self.LineTraceForTile` (+ (`self.K2_GetActorLocation`) (0.0 100.0 0.0))))
      (if _success_3
        (`KismetArrayLibrary.Array_Add` (`local.TilesFound`) _tile_3)))
    (:`then_3`
      (bind (_success_4 _tile_4) (`self.LineTraceForTile` (+ (`self.K2_GetActorLocation`) (0.0 -100.0 0.0))))
      (if _success_4
        (`KismetArrayLibrary.Array_Add` (`local.TilesFound`) _tile_4)))
    (:`then_4`
      (return (`local.TilesFound`)))))

(fn `GetTotalMovementCost`
  (returns (TotalCost :type Integer))
  (locals (Total :type Integer))
  (bind _blockage (`self.Blockage`))
  (set `local.Total` (`self.MovementCost`))
  (`/Engine/EditorBlueprintResources/StandardMacros.IsValid` _blockage
    (:`Is Valid`
      (bind _output_get (set `local.Total` (+ (`/Game/Environment/TilePlacement/Blockage.AditionalMovementCost` _blockage) (`local.Total`))))
      (return _output_get))
    (:`Is Not Valid`
      (return (`local.Total`)))))

(fn `LineTraceForTile`
  (params (TraceStart :type "Vector Structure"))
  (returns (Success :type Boolean) (Tile :type "/Game/Environment/GameMap/BP_MapTile Object Reference"))
  (bind _returnvalue (`self.GetActorUpVector`))
  (bind _outhit (`KismetSystemLibrary.LineTraceSingleForObjects` (+ TraceStart (* _returnvalue 100.0)) (+ TraceStart (* _returnvalue -1000.0)) (`|MakeArray` "ObjectTypeQuery2" :!type "EObjectTypeQuery Enum")))
  (bind _asbp_map_tile (cast `/Game/Environment/GameMap/BP_MapTile` (`.HitActor` (`GameplayStatics.BreakHitResult` _outhit)))
    (:`then`
      (return true _asbp_map_tile))
    (:`CastFailed`
      (return false null))))

(fn `SetCoordinates`
  (params (GameMapReference :type "/Game/Environment/GameMap/BP_GameMap Object Reference") (X :type Integer) (Y :type Integer))
  (set `self.GameMapReference` GameMapReference)
  (set `self.Coordinates` (`KismetMathLibrary.MakeVector2D` (`KismetMathLibrary.Conv_IntToDouble` X) (`KismetMathLibrary.Conv_IntToDouble` Y)))
  (`TextRenderComponent.K2_SetText` (`self.CoordinateText`) (`|FormatText` "{x}, {y}" X Y)))

(fn `SetHighlightMaterial`
  (if (not (`self.Void`))
    (bind _asmarker (cast `/Game/Environment/GameMap/Marker` (`ChildActorComponent.ChildActor` (`self.Marker`))))
    (`/Game/Environment/GameMap/Marker.UpdateAppearance` _asmarker self)))

(fn `UserConstructionScript`
  (`self.SetHighlightMaterial`))